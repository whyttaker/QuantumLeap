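; Blueprint function library that reads the player's saved settings from the "settings" save slot.
; GetSettings loads the SettingsSave object and returns its settings struct with a success flag.
; GetSoundSettings returns music, sound effects and dialogue volumes, each premultiplied by the master volume.
; When the save is missing or fails to cast, both report failure, and the sound volumes default to full.
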(fn `Get Settings`
  (returns (Settings :type "/Game/SettingsMenu/Blueprints/SettingsStructure Structure") (`Success?` :type Boolean))
  (bind _returnvalue (`GameplayStatics.DoesSaveGameExist` "settings"))
  (if _returnvalue
    (bind _returnvalue_2 (`GameplayStatics.LoadGameFromSlot` "settings"))
    (bind _assettings_save (cast `/Game/SettingsMenu/Blueprints/SettingsSave` _returnvalue_2)
      (:`then`
        (return (`/Game/SettingsMenu/Blueprints/SettingsSave.Settings` _assettings_save) true))
      (:`CastFailed`
        (return (struct) false)))
    (else
      (return (struct) false))))

(fn `Get Sound Settings`
  (returns (`Success?` :type Boolean) (Music :type "Float (double-precision)") (SoundFX :type "Float (double-precision)") (Dialogues :type "Float (double-precision)"))
  (bind _returnvalue (`GameplayStatics.DoesSaveGameExist` "settings"))
  (if _returnvalue
    (bind _returnvalue_2 (`GameplayStatics.LoadGameFromSlot` "settings"))
    (bind _assettings_save (cast `/Game/SettingsMenu/Blueprints/SettingsSave` _returnvalue_2)
      (:`then`
        (bind ((`MasterSound_27_08ADE772409D3AAA83FB8CBAC481B462` _mastersound) (`Music_29_09D79B214FD976A744B69D935144DE59` _music) (`SoundFX_31_D5F12AA14CDB39CBD0F4C8B1F09478F4` _soundfx) (`Dialogues_34_A8B3F31740DFFF205D5F4D80173F88C6` _dialogues)) (break `/Game/SettingsMenu/Blueprints/SettingsStructure` (`/Game/SettingsMenu/Blueprints/SettingsSave.Settings` _assettings_save)))
        (return true (* _mastersound _music) (* _mastersound _soundfx) (* _mastersound _dialogues)))
      (:`CastFailed`
        (return false 1.0 1.0 1.0)))
    (else
      (return false 1.0 1.0 1.0))))